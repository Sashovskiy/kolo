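; Player controller for polar-grid building placement that spawns a Cube actor and Build_UI.
; ChoiceBuilding checks the Building data table, deducting materials and updating cube stats upon selection, before placement.
; While selected, Tick snaps the cube's preview to angle and distance steps around world origin using the cursor trace.
; Left-click adds the tagged mesh and Sector_Circle to the cube; right-click passes the hit component to DestroyComm.
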(event EventBeginPlay
  (bind _returnvalue (Game|SpawnActorfromClass "/Game/cube.cube_C" (Math|Transform|MakeTransform "0, 0,120.000000") "Undefined" 0 0))
  (Variables|Default|SetNewVar_1 _returnvalue)
  (bind _returnvalue_2 (UserInterface|CreateWidget "/Game/Building/Build_UI.Build_UI_C"))
  (UserInterface|Viewport|AddtoViewport _returnvalue_2 0))

(event EventTick
  (params (DeltaSeconds :type Float%20%28single-precision%29))
  (bind _returnvalue (Math|Vector|MakeVector 0.0 0.0 0.0))
  (bind _returnvalue_2 (Math|Vector|MakeVector 0.0 0.0 0.0))
  (bind _hitresult (Game|Player|GetHitResultUnderCursorbyChannel "TraceTypeQuery1" true))
  (bind _constdist (Variables|Default|GetConstDist))
  (bind _newvar_1 (Variables|Default|GetNewVar_1))
  (bind _constrot (Variables|Default|GetConstRot))
  (bind _impactpoint (Collision|BreakHitResult _hitresult))
  (bind (_x _y) (Math|Vector|BreakVector _impactpoint))
  (bind _returnvalue_3 (Math|Vector|MakeVector _x _y 0.0))
  (bind _returnvalue_4 (Math|Rotator|FindLookatRotation _returnvalue_3 _returnvalue))
  (bind _returnvalue_5 (- _returnvalue_2 _returnvalue_3))
  (bind _yaw (Math|Rotator|BreakRotator _returnvalue_4))
  (bind _returnvalue_6 (Math|Vector|VectorLengthXY _returnvalue_5))
  (bind _returnvalue_7 (/ _returnvalue_6 _constdist))
  (bind _new (Utilities|To360 _yaw))
  (bind _returnvalue_8 (/ _new _constrot))
  (bind _returnvalue_9 (Math|Float|Truncate _returnvalue_7))
  (bind _returnvalue_10 (Math|Float|Truncate _returnvalue_8))
  (bind _returnvalue_11 (< _returnvalue_9 1))
  (bind _returnvalue_12 (< _returnvalue_10 1))
  (bind _returnvalue_13 (select _returnvalue_11 1 _returnvalue_9))
  (bind _returnvalue_14 (select _returnvalue_12 1 _returnvalue_10))
  (bind _returnvalue_15 (* _returnvalue_14 _constrot))
  (bind _returnvalue_16 (Math|Trig|DegreesToRadians _returnvalue_15))
  (if (!= (Variables|Default|GetSelectB) -1)
    (Development|PrintString "Hello")
    (Rendering|SetVisibility (Variables|/Game/cube.cube_C|GetStaticMesh2 _newvar_1) true false)
    (bind _sweephitresult (Transformation|SetRelativeLocationAndRotation (Variables|/Game/cube.cube_C|GetScene1 _newvar_1) (* (Math|Vector|MakeVector (* (Math|Trig|Cos(Radians) _returnvalue_16) -1.0) (* (Math|Trig|Sin(Radians) _returnvalue_16) -1.0) 0.0) (* _returnvalue_13 _constdist)) (Math|Rotator|MakeRotator 0.0 0.0 (- _yaw 1.8e+02)) false false))
    (Development|PrintString (Utilities|String|ToString(Integer) _returnvalue_13))
    (Development|PrintString (Utilities|String|ToString(Float) _returnvalue_6))
    (else
      (Development|PrintString (Utilities|GetDisplayName (.HitComponent (Collision|BreakHitResult (.HitResult (Game|Player|GetHitResultUnderCursorbyChannel "TraceTypeQuery1" true)))))))))

(event Input|MouseEvents|LeftMouseButton
  (params (Key :type Key%20Structure))
  (bind _newvar_1 (Variables|Default|GetNewVar_1))
  (bind _newvar_1_2 (Variables|Default|GetNewVar_1))
  (:Pressed
    (Rendering|SetVisibility (Variables|/Game/cube.cube_C|GetStaticMesh2 _newvar_1) false false)
    (bind _returnvalue (AddComponent|AddStaticMeshComponent _newvar_1_2 false (Transformation|GetRelativeTransform (Variables|/Game/cube.cube_C|GetScene1 _newvar_1))))
    (Components|StaticMesh|SetStaticMesh _returnvalue (Variables|Default|GetMeshPreview))
    (Utilities|Array|Add (Variables|/Script/Engine.ActorComponent|GetComponentTags _returnvalue) (Utilities|String|StringToName (Variables|Default|GetPlaceNow)))
    (Variables|Default|SetSelectB -1)
    (bind _returnvalue_2 (AddComponent|AddStaticMeshComponent _newvar_1_2 false))
    (Components|StaticMesh|SetStaticMesh _returnvalue_2 "/Game/sector_Circle.sector_Circle")
    (Transformation|AttachComponentToComponent _returnvalue_2 _returnvalue "None" "KeepRelative" "KeepRelative" "KeepRelative" true)
    (Development|PrintString (Utilities|String|Append (Utilities|String|ToString(Name) (Utilities|Array|Get(acopy) (Variables|/Script/Engine.ActorComponent|GetComponentTags _returnvalue))) " 123123"))))

(event Input|MouseEvents|RightMouseButton
  (params (Key :type Key%20Structure))
  (bind _hitresult (Game|Player|GetHitResultUnderCursorbyChannel "TraceTypeQuery1" true))
  (bind (_bblockinghit _binitialoverlap _time _distance _location _impactpoint _normal _impactnormal _physmat _hitactor _hitcomponent) (Collision|BreakHitResult _hitresult))
  (:Pressed
    (bind _ascube (Utilities|Casting|CastTocube _hitactor))
    (Default|DestroyComm _ascube _hitcomponent)))

(fn ConstructionScript)

(fn ChoiceBuilding
  (params (NewParam :type String))
  (Utilities|ChekResource NewParam
    (:Success
      (switch string NewParam
        (:Kitchen
          (Variables|Default|SetSelectB 0))
        (:MaterialMeker
          (Variables|Default|SetSelectB 1))
        (:HoleEnergy
          (Variables|Default|SetSelectB 2))
        (:SolarPanels
          (Variables|Default|SetSelectB 3))))))