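; NewGameMode is a game mode that periodically passes a platform's resource values to the game instance.
; A looping two-second timer, started on BeginPlay, finds all Cube actors and stores the first as Platform.
; Each update then calls ResourceChang, which casts to GameInst and calls Ress with that Platform's energy, material and foot values.
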(event Custom|Update
  (bind _outactors (Actor|GetAllActorsOfClass "/Game/cube.cube_C"))
  (Variables|Default|SetPlatform (Utilities|Array|Get(acopy) _outactors))
  (CallFunction|ResourceChang))

(event EventBeginPlay
  (Utilities|Time|SetTimerbyEvent (delegate Custom|Update) 2.0 true))

(event EventTick
  (params (DeltaSeconds :type Float%20%28single-precision%29)))

(fn ConstructionScript)

(fn ResourceChang
  (bind _platform (Variables|Default|GetPlatform))
  (bind _asgame_inst (Utilities|Casting|CastToGameInst (Game|GetGameInstance)))
  (Default|Ress _asgame_inst (Variables|/Game/cube.cube_C|GetEnergy _platform) (Variables|/Game/cube.cube_C|GetMaterial _platform) (Variables|/Game/cube.cube_C|GetFoot _platform)))